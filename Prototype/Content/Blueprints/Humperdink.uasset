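; Humperdink is a test Blueprint for simple movement, nudging its Ingleburt component along relative X while the R key is held.
; R press and release set a flag that Tick checks each frame.
; Tick feeds Move Component To a target slightly ahead of the current relative location, or calls its Stop input when R is up.
; Disconnected print, Lerp and range-mapping nodes are leftovers, and the construction script is empty.
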(event `self.ReceiveTick`
  (params (DeltaSeconds :type "Float (single-precision)"))
  (bind _ingleburt (`self.Ingleburt`))
  ;[1 1 1] Just testing a simple move.
  (if (`self.R_Pressed`)
    (`KismetSystemLibrary.MoveComponentTo` _ingleburt (+ (`SceneComponent.RelativeLocation` _ingleburt) (2.0 0.0 0.0)) :!label _label)
    (else
      (goto _label :!via `Stop`))))

(event `Key|R`
  ;[1 1 1] Just testing a simple move.
  (:`Pressed`
    (set `self.R_Pressed` true))
  (:`Released`
    (set `self.R_Pressed` false)))

(fn `UserConstructionScript`)